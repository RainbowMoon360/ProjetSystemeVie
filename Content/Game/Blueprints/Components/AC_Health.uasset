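; AC_Health is an actor component that tracks an owner's health and death state.
; TakeDamage and GainHealth adjust health while alive and print the new value; ResetHealth restores it to max and clears the dead flag.
; All three route through UpdateHealthAndNotify, which clamps health, broadcasts OnHealthChanged, and sets IsDead and fires OnDeath at zero.
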(event EventTakeDamage
  (params (DamageNumber :type Float%20%28double-precision%29))
  (if (not (Variables|Default|GetIsDead))
    (CallFunction|UpdateHealthandNotify (- (Variables|Default|GetCurrentHealth) DamageNumber))
    (Development|PrintString (Utilities|String|ToString(Float) (Variables|Default|GetCurrentHealth)))))

(event EventGainHealth
  (params (HealthAmount :type Float%20%28double-precision%29))
  (if (not (Variables|Default|GetIsDead))
    (CallFunction|UpdateHealthandNotify (+ (Variables|Default|GetCurrentHealth) HealthAmount))
    (Development|PrintString (Utilities|String|ToString(Float) (Variables|Default|GetCurrentHealth)))))

(event EventResetHealth
  (Variables|Default|SetIsDead false)
  (CallFunction|UpdateHealthandNotify (Variables|Default|GetMaxHealth)))

(fn UpdateHealthandNotify
  (params (NewHealthValue :type Float%20%28double-precision%29))
  (bind _maxhealth (Variables|Default|GetMaxHealth))
  ;[0.15 0.15 0.15 0.5] Update health variables in AC_Health. Invoking OnHealthChange to inform listeners that health changed. Invoking OnDeath if health is 0.
  (bind _output_get (Variables|Default|SetCurrentHealth (Math|Float|Clamp(Float) NewHealthValue 0.0 _maxhealth)))
  (Default|CallOnHealthChanged _output_get _maxhealth)
  (if (<= (Variables|Default|GetCurrentHealth) 0.0)
    (Variables|Default|SetIsDead true)
    (Default|CallOnDeath)
    (else
      (Variables|Default|SetIsDead false))))